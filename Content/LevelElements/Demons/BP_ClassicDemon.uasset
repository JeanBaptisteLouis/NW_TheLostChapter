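; Demon enemy that tracks the player and fires demon bullets at them.
; Each tick the head turns toward player character 0 with pitch held at zero, while an arrow component takes the full look-at rotation as the aim.
; BeginPlay starts a looping timer for periodic shooting.
; The shoot function spawns BP_DemonBullet at the arrow's transform only when a visibility trace from the arrow hits the player.
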(event EventTick
  (params (DeltaSeconds :type Float%20%28single-precision%29))
  (bind _returnvalue (Game|GetPlayerCharacter 0))
  (bind _head (Variables|Default|GetHead))
  (bind _returnvalue_2 (Transformation|GetWorldLocation _head))
  (bind _returnvalue_3 (Transformation|GetActorLocation _returnvalue))
  (bind _returnvalue_4 (Math|Rotator|FindLookatRotation _returnvalue_2 _returnvalue_3))
  (Transformation|SetWorldRotation (Variables|Default|GetHead) (Math|Rotator|MakeRotator (.roll _returnvalue_4) 0.0 (.yaw _returnvalue_4)) false false)
  (Transformation|SetWorldRotation (Variables|Default|GetArrow) (Math|Rotator|MakeRotator (.roll _returnvalue_4) (.pitch _returnvalue_4) (.yaw _returnvalue_4)) false false))

(event EventBeginPlay
  (bind _returnvalue (Utilities|Time|SetTimerbyEvent (EventDispatchers|CreateEvent :!event FCTShoot) 2.0 true))
  (Variables|Default|SetShootingTimerHandler _returnvalue))

(fn ConstructionScript
  (|CallParentFunction))

(fn FCTShoot
  (bind _outhit (Collision|LineTraceByChannel (Transformation|GetWorldLocation (Variables|Default|GetArrow)) (Transformation|GetActorLocation (Game|GetPlayerCharacter 0)) "TraceTypeQuery1" false 0 "None"))
  (if (== (.hitactor _outhit) (Game|GetPlayerCharacter 0))
    (Game|SpawnActorfromClass "/Game/Cards/Bullets/BP_DemonBullet.BP_DemonBullet_C" (Transformation|GetWorldTransform (Variables|Default|GetArrow)) "Undefined" "MultiplyWithRoot" 0 "NewEnumerator4" 0 0)))