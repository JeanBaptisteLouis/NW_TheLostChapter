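; BP_DemonParent is the base Blueprint for demons, handling their health and death.
; Taking damage reduces Life and triggers death once it reaches zero or below.
; On death it spawns its CardLoot, if set, at the CardLootPoint transform, then notifies every actor implementing BPI_DemonsCont through an interface message before destroying itself.
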(fn ConstructionScript)

(fn FCTTakeDamage
  (params (DamageAmmount :type Integer))
  (bind _output_get (Variables|Basics|SetLife (- (Variables|Basics|GetLife) DamageAmmount)))
  (if (<= _output_get 0)
    (CallFunction|FCTDeath)
    (return)
    (else
      (return))))

(fn FCTDeath
  (bind _cardloot (Variables|Basics|GetCardLoot)
    (:then
      (Game|SpawnActorfromClass _cardloot (Transformation|GetWorldTransform (Variables|Default|GetCardLootPoint)) "Undefined" "MultiplyWithRoot" 0 0))
    (:else
      _))
  (bind _outactors (Actor|GetAllActorswithInterface "/Game/LevelElements/Demons/BPI_DemonsCont.BPI_DemonsCont_C"))
  (for _array_element _outactors
    (Class|BPIDemonsCont|FCTIonDemonDeath(Message) _array_element))
  (Actor|DestroyActor))