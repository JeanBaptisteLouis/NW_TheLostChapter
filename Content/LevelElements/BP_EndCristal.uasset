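; BP_EndCristal is the level exit crystal, unlocked once every demon in the level is dead.
; On BeginPlay it gathers all BP_DemonParent actors and shows their count on a text component.
; Each demon death event updates the remaining count, and the last one destroys the text and sets CanFinish.
; When the first-person character then overlaps the crystal, it pauses the game and shows the W_LevelComplete widget.
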(event OnComponentBeginOverlap(Cristal)
  (params (OverlappedComponent :type Primitive%20Component%20Object%20Reference) (OtherActor :type Actor%20Object%20Reference) (OtherComp :type Primitive%20Component%20Object%20Reference) (OtherBodyIndex :type Integer) (bFromSweep :type Boolean) (SweepResult :type Hit%20Result%20Structure%20%28by%20ref%29))
  (Utilities|Casting|CastToBP_FirstPersonCharacter OtherActor)
  (CallFunction|Finish))

(event Custom|Finish
  (if (Variables|Default|GetbCanFinish)
    (Game|SetGamePaused true)
    (bind _returnvalue (UserInterface|CreateWidget "/Game/UI/W_LevelComplete.W_LevelComplete_C"))
    (UserInterface|Viewport|AddtoViewport _returnvalue 0)))

(event EventBeginPlay
  (bind _outactors (Actor|GetAllActorsOfClass "/Game/LevelElements/Demons/BP_DemonParent.BP_DemonParent_C"))
  (Variables|Default|SetDemons _outactors)
  (Rendering|Components|TextRender|SetText (Variables|Default|GetLeftDemonsText) (Utilities|Text|ToText(Integer) (Utilities|Array|Length (Variables|Default|GetDemons)))))

(event EventFCTIonDemonDeath
  (bind _result (Math|Integer|IncrementInt (Variables|Default|GetDeadDemonsNB))
    (:%20%20
      (if (== _result (Utilities|Array|Length (Variables|Default|GetDemons)))
        (Variables|Default|SetbCanFinish true)
        (Components|DestroyComponent (Variables|Default|GetLeftDemonsText))
        (else
          (CallFunction|FCTUpadteLeftDemonsText))))))

(fn ConstructionScript)

(fn FCTUpadteLeftDemonsText
  (Rendering|Components|TextRender|SetText (Variables|Default|GetLeftDemonsText) (Utilities|Text|ToText(Integer) (- (Utilities|Array|Length (Variables|Default|GetDemons)) (Variables|Default|GetDeadDemonsNB)))))