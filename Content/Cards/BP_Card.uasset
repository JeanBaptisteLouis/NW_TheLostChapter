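; Card actor for a weapon card, deriving its type (Slash, Glock or AK) from its class name at construction.
; BeginPlay loads max ammo and color from the DB_Cards table and tints the mesh.
; Tick brightens the front card's material, and Fire drives a timeline scale pulse.
; Discard attaches it to the player camera, drifts the mesh with a timeline, then destroys it; the ability is only a debug print.
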(event Custom|Discard
  (params (useAbility :type Boolean))
  (Utilities|FlowControl|Sequence
    (:then_0
      (if useAbility
        (Development|PrintString "POWAAAA")))
    (:then_1
      (Variables|Default|Setdiscarding true)
      (Transformation|AttachComponentToComponent (Variables|/Game/FirstPerson/Blueprints/BP_FirstPersonCharacter.BP_FirstPersonCharacter_C|GetFirstPersonCamera (.AsBP%20First%20Person%20Character (Utilities|Casting|CastToBP_FirstPersonCharacter (Game|GetPlayerCharacter 0)))) "None" "KeepWorld" "KeepWorld" "KeepWorld" true)
      (bind _alpha (Timeline|discardTM PlayFromStart)
        (:Update
          (Transformation|AddRelativeLocation (Variables|Default|GetMesh) (Math|Vector|MakeVector (* (Utilities|Time|GetWorldDeltaSeconds) 2e+01 (- 1.0 _alpha)) (* (Utilities|Time|GetWorldDeltaSeconds) 2e+01 (- 1.0 _alpha)) (* (Utilities|Time|GetWorldDeltaSeconds) 2e+01 (- 1.0 _alpha))) false false))
        (:Finished
          (Actor|DestroyActor))))))

(event Custom|Fire
  (bind _newtrack_0 (Timeline|fireTM PlayFromStart)
    (:Update
      (Transformation|SetWorldScale3D (Variables|Default|GetMesh) (Math|Conversions|ToVector(Float) (+ (/ _newtrack_0 1e+01) 1.0))))))

(event EventBeginPlay
  (bind _returnvalue (Utilities|GetDataTableRow "/Game/Cards/DB_Cards.DB_Cards" (Utilities|String|StringToName (Utilities|String|EnumtoString (Variables|Default|GetCard%20Typer))))
    (:then
      (Variables|Ammo|SetmaxAmmo (.maxammo _returnvalue))
      (bind _output_get (Variables|Default|Setcolor (.color _returnvalue)))
      (Rendering|Material|SetVectorParameterValueonMaterials (Variables|Default|GetMesh) "Color" (Math|Conversions|ToVector(LinearColor) _output_get)))))

(event Collision|EventActorBeginOverlap
  (params (OtherActor :type Actor%20Object%20Reference)))

(event EventTick
  (params (DeltaSeconds :type Float%20%28single-precision%29))
  (if (not (Variables|Default|Getdiscarding))
    (bind _output_get (Variables|Default|SetlightValue (Math|Interpolation|FInterpTo (Variables|Default|GetlightValue) (Math|Float|SelectFloat 1.0 0.3 (Variables|Default|GetonFront)) DeltaSeconds 15.0)))
    (Rendering|Material|SetScalarParameterValueonMaterials (Variables|Default|GetMesh) "Intensity" _output_get)))

(fn ConstructionScript
  (bind _self self)
  (bind _returnvalue (Utilities|GetClass _self))
  (bind _returnvalue_2 (Utilities|GetClassDisplayName _returnvalue))
  (if (Utilities|String|Contains _returnvalue_2 "Slash" false true)
    (Variables|Default|SetCard%20Typer "NewEnumerator2")
    (elif (Utilities|String|Contains _returnvalue_2 "Glock" false true)
      (Variables|Default|SetCard%20Typer "NewEnumerator0")
      (elif (Utilities|String|Contains _returnvalue_2 "AK" false true)
        (Variables|Default|SetCard%20Typer "NewEnumerator3")))))