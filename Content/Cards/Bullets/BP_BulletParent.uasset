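; BP_BulletParent is the base projectile for card weapon types such as Slash, Glock, AK and Demon.
; Construction adds slight random pitch and yaw spread for AK only, and tints the mesh with the color from the DB_Cards row matching its Type.
; A sphere hit spawns an N_Hit effect, passes Damage to any BP_DemonParent struck, then destroys the bullet.
; Its own FTakeDamage event also destroys it.
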(event OnComponentHit(Sphere)
  (params (HitComponent :type Primitive%20Component%20Object%20Reference) (OtherActor :type Actor%20Object%20Reference) (OtherComp :type Primitive%20Component%20Object%20Reference) (NormalImpulse :type Vector :default "0, 0, 0") (Hit :type Hit%20Result%20Structure%20%28by%20ref%29))
  (Niagara|SpawnSystematLocation "/Game/VFX/N_Hit.N_Hit" (.location Hit) (Math|Conversions|RotationFromXVector (.normal Hit)))
  (bind _asbp_demon_parent (Utilities|Casting|CastToBP_DemonParent OtherActor)
    (:then
      (Default|FCTTakeDamage _asbp_demon_parent (Variables|Default|GetDamage))
      (Actor|DestroyActor))
    (:CastFailed
      (Actor|DestroyActor))))

(event EventBeginPlay)

(event EventFTakeDamage
  (params (amount :type Integer))
  (Actor|DestroyActor))

(fn ConstructionScript
  (bind _returnvalue (Math|Random|RandomUnitVector))
  (bind _type (Variables|Default|GetType))
  (bind _returnvalue_2 (Utilities|Select :Index _type :NewEnumerator2 0.0 :NewEnumerator0 0.0 :NewEnumerator3 1.0 :NewEnumerator4 0.0))
  (bind _returnvalue_3 (* _returnvalue _returnvalue_2))
  (Class|Actor|AddActorWorldRotation (Math|Rotator|MakeRotator 0.0 (.x _returnvalue_3) (.y _returnvalue_3)))
  (bind _returnvalue_4 (Utilities|GetDataTableRow "/Game/Cards/DB_Cards.DB_Cards" (Utilities|String|StringToName (Utilities|String|EnumtoString (Variables|Default|GetType))))
    (:then
      (Rendering|Material|SetVectorParameterValueonMaterials (Variables|Default|GetMesh) "Color" (Math|Conversions|ToVector(LinearColor) (.color _returnvalue_4))))))