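; BP_AK_ball is an explosive ball projectile that damages nearby actors and can blast the player away.
; On hit, its sphere stops simulating physics and a timeline inflates it before detonation.
; It then launches the player away with an upward-biased direction, or with zero velocity outside Radius, overriding current velocity either way.
; Finally, it sends a damage message to actors found by a sphere overlap and destroys itself.
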(event OnComponentHit(Sphere)
  (params (HitComponent :type Primitive%20Component%20Object%20Reference) (OtherActor :type Actor%20Object%20Reference) (OtherComp :type Primitive%20Component%20Object%20Reference) (NormalImpulse :type Vector :default "0, 0, 0") (Hit :type Hit%20Result%20Structure%20%28by%20ref%29))
  (bind _returnvalue (Transformation|GetActorLocation))
  (bind _player (Variables|Default|Getplayer))
  (bind _firstpersoncamera (Variables|/Game/FirstPerson/Blueprints/BP_FirstPersonCharacter.BP_FirstPersonCharacter_C|GetFirstPersonCamera _player))
  (bind _returnvalue_2 (Transformation|GetWorldLocation _firstpersoncamera))
  (bind _returnvalue_3 (- _returnvalue_2 _returnvalue))
  (Physics|SetSimulatePhysics (Variables|Default|GetSphere) false)
  (bind _alpha (Timeline|explode PlayFromStart)
    (:Update
      (Transformation|SetWorldScale3D (Variables|Default|GetSphere) (Math|Conversions|ToVector(Float) (+ _alpha 1.0))))
    (:Finished
      (Character|LaunchCharacter _player (* (Math|Float|SelectFloat 1.5e+03 0.0 (< (Math|Vector|VectorLength _returnvalue_3) (Variables|Default|Getradius))) (Math|Vector|Normalize (* _returnvalue_3 "0.500000,0.500000,1.000000"))) true true)
      (bind _outactors (Collision|SphereOverlapActors (Transformation|GetActorLocation) 5e+02 (Variables|Default|GetObject%20Types) 0))
      (for _array_element _outactors
        (Class|BPIDamage|FTakeDamage(Message) _array_element 8))
      (Actor|DestroyActor))))

(event EventBeginPlay
  (|CallParentFunction) ; This node is disabled and will not be called.\nDrag off pins to build functionality.
)

(event Collision|EventActorBeginOverlap
  (params (OtherActor :type Actor%20Object%20Reference)))

(event EventTick
  (params (DeltaSeconds :type Float%20%28single-precision%29)))

(fn ConstructionScript
  (|CallParentFunction))