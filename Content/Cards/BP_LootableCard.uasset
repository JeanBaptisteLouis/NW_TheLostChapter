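; BP_LootableCard is a world pickup that gives the player a card of its CardType.
; On BeginPlay it looks up that type's row in the DB_Cards data table and tints the card mesh with the row's color.
; Every tick it smoothly rotates to face the player.
; When the player overlaps its sphere, it calls Draw on the player's hand component and destroys itself.
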(event OnComponentBeginOverlap(Sphere)
  (params (OverlappedComponent :type Primitive%20Component%20Object%20Reference) (OtherActor :type Actor%20Object%20Reference) (OtherComp :type Primitive%20Component%20Object%20Reference) (OtherBodyIndex :type Integer) (bFromSweep :type Boolean) (SweepResult :type Hit%20Result%20Structure%20%28by%20ref%29))
  (bind _player (Variables|Default|GetPlayer))
  (if (== OtherActor _player)
    (Default|Draw (Variables|/Game/FirstPerson/Blueprints/BP_FirstPersonCharacter.BP_FirstPersonCharacter_C|GetBPC_Hand _player) (Variables|Default|GetCard%20Type))
    (Actor|DestroyActor)))

(event EventBeginPlay
  (bind _asbp_first_person_character (Utilities|Casting|CastToBP_FirstPersonCharacter (Game|GetPlayerCharacter 0))
    (:then
      (Variables|Default|SetPlayer _asbp_first_person_character))
    (:CastFailed
      _))
  (bind _returnvalue (Utilities|GetDataTableRow "/Game/Cards/DB_Cards.DB_Cards" (Utilities|String|StringToName (Utilities|String|EnumtoString (Variables|Default|GetCard%20Type))))
    (:then
      (Rendering|Material|SetVectorParameterValueonMaterials (Variables|Default|GetCardMesh) "Color" (Math|Conversions|ToVector(LinearColor) (.color _returnvalue))))))

(event Collision|EventActorBeginOverlap
  (params (OtherActor :type Actor%20Object%20Reference)))

(event EventTick
  (params (DeltaSeconds :type Float%20%28single-precision%29))
  (bind _scene (Variables|Default|GetScene))
  (Transformation|SetWorldRotation _scene (Math|Interpolation|RInterpTo (Transformation|GetWorldRotation _scene) (Math|Rotator|FindLookatRotation (Transformation|GetActorLocation) (Transformation|GetActorLocation (Variables|Default|GetPlayer))) DeltaSeconds 1e+01) false false))

(fn ConstructionScript)